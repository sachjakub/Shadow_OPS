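; Teleporter pad that sends any actor overlapping its box to a randomly chosen pad, possibly itself.
; Each pad registers in the GameInstance's Teleports array on BeginPlay, and the actor lands slightly above the chosen pad with zeroed rotation.
; The triggered pad then enters a random-length cooldown, swapping its cylinder material from pulsing to static until a timer re-arms it.
; Only the triggered pad cools down, not the destination.
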(event `self.ReceiveBeginPlay`
  (bind _asmy_game_instance (cast `/Game/Blueprints/MyGameInstance` (`GameplayStatics.GetGameInstance`)))
  (`KismetArrayLibrary.Array_Append` (`/Game/Blueprints/MyGameInstance.Teleports` _asmy_game_instance) (`|MakeArray` self :!type "/Game/Blueprints/BPTeleport Object Reference")))

(event `self.Box.OnComponentBeginOverlap`
  (params (OverlappedComponent :type "PrimitiveComponent Object Reference") (OtherActor :type "Actor Object Reference") (OtherComp :type "PrimitiveComponent Object Reference") (OtherBodyIndex :type Integer) (bFromSweep :type Boolean) (SweepResult :type "HitResult Structure (by ref)"))
  (if (not (`self.cooldown`))
    (bind _asmy_game_instance (cast `/Game/Blueprints/MyGameInstance` (`GameplayStatics.GetGameInstance`)))
    (bind _teleports (`/Game/Blueprints/MyGameInstance.Teleports` _asmy_game_instance))
    (`self.K2_TeleportTo` :`self` OtherActor :`DestLocation` (+ (`self.K2_GetActorLocation` (`|GetArrayItem` _teleports (`KismetMathLibrary.RandomIntegerInRange` 0 (`KismetArrayLibrary.Array_LastIndex` _teleports)))) (0.0 0.0 10.0)))
    (set `self.cooldown` true)
    (`KismetSystemLibrary.K2_SetTimer` null "cooledDown" (`KismetMathLibrary.RandomFloatInRange` 3.0 20.0))
    (`PrimitiveComponent.SetMaterial` (`self.Cylinder`) 0 "/Game/StarterContent/Materials/M_Tech_Hex_Tile.M_Tech_Hex_Tile")))

(event `cooledDown`
  (set `self.cooldown` false)
  (`PrimitiveComponent.SetMaterial` (`self.Cylinder`) 0 "/Game/StarterContent/Materials/M_Tech_Hex_Tile_Pulse.M_Tech_Hex_Tile_Pulse"))

(fn `UserConstructionScript`)